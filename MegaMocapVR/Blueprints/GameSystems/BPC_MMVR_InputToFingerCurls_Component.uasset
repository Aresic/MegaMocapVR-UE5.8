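; Actor component for the MMVR VR player pawn that turns thumb, index and grip input events into animated finger curls for both hands.
; A latent macro eases each on/off input toward 0 or 1 frame by frame, with grip driving middle, ring and pinky together.
; Tick sends the curls, zero splay and a sine-based breathing value to the pawn.
; SteamVR curl tracking is a disabled stub retained for future Index/Knuckles support.
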(event Custom|Event_InputEvent
  (params (Finger_Enum :type MMVR_InputFinger%20Enum :default "NewEnumerator0") (InputOn :type Boolean) (HandLeft :type Boolean))
  (if (Variables|Default|GetIsEnabled)
    (if HandLeft
      (switch Utilities|FlowControl|Switch|SwitchonMMVR_InputFinger Finger_Enum
        (:NewEnumerator0
          (Variables|Default|SetLThumbCurled InputOn)
          (Utilities|BooltoFInterpFloat (Variables|Default|GetLThumbCurled) (Variables|Default|GetLThumb_Float) 16.0) ; enters at Start
        )
        (:NewEnumerator1
          (Variables|Default|SetLIndexCurled InputOn)
          (Utilities|BooltoFInterpFloat (Variables|Default|GetLIndexCurled) (Variables|Default|GetLIndex_Float) 16.0) ; enters at Start
        )
        (:NewEnumerator10
          (Variables|Default|SetLGripCurled InputOn)
          (Utilities|BooltoFInterpFloat (Variables|Default|GetLGripCurled) (Variables|Default|GetLGrip_Float) 16.0) ; enters at Start
        ))
      (else
        (switch Utilities|FlowControl|Switch|SwitchonMMVR_InputFinger Finger_Enum
          (:NewEnumerator0
            (Variables|Default|SetRThumbCurled InputOn)
            (Utilities|BooltoFInterpFloat (Variables|Default|GetRThumbCurled) (Variables|Default|GetRThumb_Float) 16.0) ; enters at Start
          )
          (:NewEnumerator1
            (Variables|Default|SetRIndexCurled InputOn)
            (Utilities|BooltoFInterpFloat (Variables|Default|GetRIndexCurled) (Variables|Default|GetRIndex_Float) 16.0) ; enters at Start
          )
          (:NewEnumerator10
            (Variables|Default|SetRGripCurled InputOn)
            (Utilities|BooltoFInterpFloat (Variables|Default|GetRGripCurled) (Variables|Default|GetRGrip_Float) 16.0) ; enters at Start
          ))))))

(event EventBeginPlay
  (bind _asmmvr_player_pawn_bp (Utilities|Casting|CastToMMVR_PlayerPawn_BP (Components|GetOwner)))
  (Variables|Default|SetAs%20MMVR%20Player%20Pawn%20BP _asmmvr_player_pawn_bp))

(event EventTick
  (params (DeltaSeconds :type Float%20%28single-precision%29))
  (bind _lgrip_float (Variables|Default|GetLGrip_Float))
  (bind _rgrip_float (Variables|Default|GetRGrip_Float))
  (if (Variables|Default|GetIsEnabled)
    (bind _output_get (Variables|Default|SetFingerCurls_Struct (Utilities|Struct|MakeSteamVR_fingerCurls_Struct (Variables|Default|GetLThumb_Float) (Variables|Default|GetLIndex_Float) _lgrip_float _lgrip_float _lgrip_float (Variables|Default|GetRThumb_Float) (Variables|Default|GetRIndex_Float) _rgrip_float _rgrip_float _rgrip_float 0.0 0.0 0.0 0.0 0.0 0.0 0.0 0.0 0.0 0.0)))
    (Default|SendFingerData (Variables|Default|GetAs%20MMVR%20Player%20Pawn%20BP) _output_get (Math|Float|Clamp(Float) (Math|Float|Absolute(Float) (Math|Trig|Sin(Radians) (* (Utilities|Time|GetGameTimeinSeconds) 1.0)))))))

(fn UpdateSteamVRFingerCurls
  (params (Hand :type EControllerHand%20Enum :default "Left")))

(fn MMVR
  (return ""))