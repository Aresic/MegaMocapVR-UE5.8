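; VR quick-select menu actor with four directional buttons, which scales in and out when toggled for a controller hand.
; While it is open, Tick moves a tracker to the hand and sets the hovered-button enum from its dominant local X/Z offset past a dead zone.
; The enum's RepNotify drives timeline hover animations (material, position, child transform) and controller haptics.
; MMVR_ConsumeQuickSelection returns the current choice and clears the menu state.
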(event Custom|QuickSelectMenu_Toggle
  (params (SpawnedHand :type Actor%20Component%20Object%20Reference) (ToggleOn :type Boolean) (IsLeftHand? :type Boolean) (ButtonUVOffsetY :type Float%20%28double-precision%29) (MakeMenuInvisible :type Boolean))
  (bind _returnvalue (not MakeMenuInvisible))
  (bind _returnvalue_2 (and ToggleOn _returnvalue))
  (if (or (not (Variables|Default|GetMenuOn)) (not ToggleOn))
    (Utilities|ResetButtonParameters ButtonUVOffsetY)
    (Variables|Default|SetSpawned%20Hand SpawnedHand)
    (Rendering|SetVisibility (Variables|Default|GetQuickSelectMenu_Root) _returnvalue_2 true)
    (if _returnvalue_2
      (Variables|Default|SetQuickMenu%20Enum "NewEnumerator6")
      (Variables|Default|SetMenuOn true)
      (bind _newtrack_0 (Timeline|Timeline_1 PlayFromStart)
        (:Update
          (Transformation|SetWorldScale3D (Variables|Default|GetQuickSelectMenu_Root) (Math|Conversions|ToVector(Float) _newtrack_0))))
      (else
        (Variables|Default|SetMenuOn false)
        (Variables|Default|SetQuickMenu%20Enum "NewEnumerator6")
        (Timeline|Timeline_1 ReverseFromEnd)))))

(event Custom|ButtonToggleOff
  (params (ButtonStatic%20Mesh :type Static%20Mesh%20Component%20Object%20Reference))
  (bind _output_get (Variables|Default|SetOldButton_Hover ButtonStatic%20Mesh))
  (bind _newtrack_0 (Timeline|Timeline_2 ReverseFromEnd)
    (:Update
      (Utilities|AnimateUI _newtrack_0 _output_get))))

(event Custom|ButtonToggleOn
  (params (ButtonStaticMesh :type Static%20Mesh%20Component%20Object%20Reference))
  (bind _returnvalue (Game|GetPlayerController 0))
  (bind _newtrack_0 (Timeline|Timeline_3 PlayFromStart)
    (:Update
      (Utilities|AnimateUI _newtrack_0 (Variables|Default|GetNewButton_Hover))
      (if (Utilities|String|Contains (Utilities|String|ToString(Object) (Variables|Default|GetSpawned%20Hand)) "HandControllerL")
        ;[1 1 1] put haptics here
        (Class|PlayerController|PlayHapticEffect _returnvalue "/Game/MegaMocapVR/Blueprints/GameSystems/Input/HapticFeedback_MenuSelect.HapticFeedback_MenuSelect" "Left" 1.0 false)
        (else
          (Class|PlayerController|PlayHapticEffect _returnvalue "/Game/MegaMocapVR/Blueprints/GameSystems/Input/HapticFeedback_MenuSelect.HapticFeedback_MenuSelect" "Right" 1.0 false))))))

(event EventBeginPlay
  (Variables|Default|SetButtonRelativeOrigin (Variables|/Script/Engine.SceneComponent|GetRelativeLocation (Variables|Default|GetDownButton_BG)))
  (Transformation|SetWorldScale3D (Variables|Default|GetQuickSelectMenu_Root) "0, 0, 0"))

(event Collision|EventActorBeginOverlap
  (params (OtherActor :type Actor%20Object%20Reference)))

(event EventTick
  (params (DeltaSeconds :type Float%20%28single-precision%29))
  (if (and (Variables|Default|GetMenuOn) (Rendering|IsVisible (Variables|Default|GetQuickSelectMenu_Root)))
    (Utilities|FlowControl|Sequence
      (:then_0
        (Utilities|UpdateControllerTrackerLocation))
      (:then_1
        (Utilities|DetermineWhichButtonHover)))
    (elif (Variables|Default|GetMenuOn)
      (Variables|Default|SetMenuOn false)
      (Variables|Default|SetQuickMenu%20Enum "NewEnumerator6"))))

(fn ConstructionScript)

(fn SmoothControllerPosition
  (params (LiveLinkTransformBlueprintData :type Live%20Link%20Transform%20Blueprint%20Data%20Structure%20%28by%20ref%29))
  (bind _framedata (Utilities|Struct|BreakLiveLinkTransformBlueprintData LiveLinkTransformBlueprintData))
  (bind _transform (Utilities|Struct|BreakLiveLinkTransformFrameData _framedata))
  (bind (_location _rotation) (Math|Transform|BreakTransform _transform))
  (bind _output_get (LocalVariables|SetController%20Previous%20Frame%20Location (Class|KismetMathLibrary|WeightedMovingAverageFVector _location (LocalVariables|GetController%20Previous%20Frame%20Location) 0.7)))
  (bind _output_get_2 (LocalVariables|SetController%20Previous%20Frame%20Rotation (Class|KismetMathLibrary|WeightedMovingAverageFRotator _rotation (LocalVariables|GetController%20Previous%20Frame%20Rotation) 0.7)))
  (return _output_get _output_get_2))

(fn OnRepQuickMenuEnum
  (Utilities|IsValid (Variables|Default|GetNewButton_Hover)
    (:Is%20Valid
      (CallFunction|ButtonToggleOff (Variables|Default|GetNewButton_Hover)))
    (:Is%20Not%20Valid
      _))
  (switch Utilities|FlowControl|Switch|SwitchonMMVRQuickMenu_ButtonHover_Enum (Variables|Default|GetQuickMenu%20Enum)
    (:NewEnumerator6
      (Variables|Default|SetNewButton_Hover 0))
    (:NewEnumerator0
      (Variables|Default|SetNewButton_Hover (Variables|Default|GetUpButton_BG)))
    (:NewEnumerator1
      (Variables|Default|SetNewButton_Hover (Variables|Default|GetRightButton_BG)))
    (:NewEnumerator3
      (Variables|Default|SetNewButton_Hover (Variables|Default|GetDownButton_BG)))
    (:NewEnumerator7
      (Variables|Default|SetNewButton_Hover (Variables|Default|GetLeftButton_BG))))
  (CallFunction|ButtonToggleon (Variables|Default|GetNewButton_Hover)))

(fn MMVRConsumeQuickSelection
  (if (and (Variables|Default|GetMenuOn) (Rendering|IsVisible (Variables|Default|GetQuickSelectMenu_Root)))
    (Variables|Default|SetMMVR_ConsumedSelection (Variables|Default|GetQuickMenu%20Enum))
    (else
      (Variables|Default|SetMMVR_ConsumedSelection "NewEnumerator6")))
  (Variables|Default|SetMenuOn false)
  (Variables|Default|SetQuickMenu%20Enum "NewEnumerator6")
  (return (Variables|Default|GetMMVR_ConsumedSelection)))